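; BP_Leaderboard submits the race result to a leaderboard REST API and shows the top ten on the race end screen.
; It binds to RedisRacerGameMode's race end event, then uses VaRest to POST the score and initials to a localhost server.
; The GET fires immediately without waiting for the POST, fills a ranked map, then creates W_RaceEnd.
; Failed requests only print the response, so a failed GET shows no widget.
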(event Custom|AddLeaderboardEntry
  ;[0.15 0.15 0.15 0.5] RestAPI: AddLeaderboardEntry
  (bind _returnvalue (Class|VaRestSubsystem|ConstructVaRestRequestExt (|VaRestSubsystem) "POST" "json"))
  (Class|VaRestRequestJSON|SetRequestObject _returnvalue (|MakeJson (Variables|Default|GetLeaderboardKey) (Utilities|String|ToString(Integer) (Variables|Default|GetScore)) (Variables|Default|GetInitials)))
  (Class|VaRestRequestJSON|ProcessURL _returnvalue "http://localhost:3000/api/leaderboard")
  (EventDispatchers|BindEventtoOnRequestFail _returnvalue (delegate Custom|AddLeaderboardEntryRequest))
  (EventDispatchers|BindEventtoOnRequestComplete _returnvalue (delegate Custom|AddLeaderboardEntryRequest)))

(event Custom|GetLeaderboard
  ;[0.15 0.15 0.15 0.5] RestAPI: GetLeaderboard
  (bind _returnvalue (Class|VaRestSubsystem|ConstructVaRestRequestExt (|VaRestSubsystem) "GET" "json"))
  (Class|VaRestRequestJSON|ProcessURL _returnvalue "http://localhost:3000/api/leaderboard/redis-racer?count=10")
  (EventDispatchers|BindEventtoOnRequestFail _returnvalue (delegate Custom|GetLeaderboardFail))
  (EventDispatchers|BindEventtoOnRequestComplete _returnvalue (delegate Custom|GetLeaderboardComplete)))

(event Custom|CreateRaceEndWidget
  ;[0.15 0.15 0.15 0.5] CreateRaceEndWidget
  (bind _returnvalue (UserInterface|CreateWidget "/Game/Blueprints/Widgets/W_RaceEnd.W_RaceEnd_C" 0 (Variables|Default|GetWin) (Variables|Default|GetLeaderboard) (Variables|Default|GetScore)))
  (UserInterface|Viewport|AddtoViewport _returnvalue 0))

(event Custom|RaceEnd
  (params (Win :type Boolean) (Score :type Integer) (Initials :type String))
  ;[0.15 0.15 0.15 0.5] EventBeginPlay
  (Variables|Default|SetWin Win)
  (Variables|Default|SetScore Score)
  (Variables|Default|SetInitials Initials)
  (CallFunction|AddLeaderboardEntry)
  (CallFunction|GetLeaderboard))

(event Custom|AddLeaderboardEntryRequest
  (params (Request :type Va%20Rest%20Request%20JSON%20Object%20Reference))
  ;[0.15 0.15 0.15 0.5] RestAPI: AddLeaderboardEntry
  (bind _returnvalue (Class|VaRestRequestJSON|GetResponseContentasString Request true))
  (Development|PrintString _returnvalue))

(event Custom|GetLeaderboardFail
  (params (Request :type Va%20Rest%20Request%20JSON%20Object%20Reference))
  ;[0.15 0.15 0.15 0.5] RestAPI: GetLeaderboard
  (bind _returnvalue (Class|VaRestRequestJSON|GetResponseContentasString Request true))
  (Development|PrintString _returnvalue))

(event Custom|GetLeaderboardComplete
  (params (Request :type Va%20Rest%20Request%20JSON%20Object%20Reference))
  ;[0.15 0.15 0.15 0.5] RestAPI: GetLeaderboard
  ;;[0.15 0.15 0.15 0.5] GetLeaderboardComplete
  (for (_array_element _array_index) (|BreakJson (Class|VaRestRequestJSON|GetResponseObject Request))
    (Utilities|Map|Add (Variables|Default|GetLeaderboard) (Utilities|String|Append (Utilities|String|ToString(Integer) (+ _array_index 1)) ") " (Utilities|String|Left (Class|VaRestJsonObject|GetStringField _array_element "value") 3)) (Class|VaRestJsonObject|GetIntegerField _array_element "score")))
  (CallFunction|CreateRaceEndWidget))

(event EventBeginPlay
  ;[0.15 0.15 0.15 0.5] EventBeginPlay
  (bind _asredis_racer_game_mode (Utilities|Casting|CastToRedisRacerGameMode (Game|GetGameMode)))
  (bind _output_get (Variables|Default|SetRedisRacerGM _asredis_racer_game_mode))
  (EventDispatchers|BindEventtoEventRaceEnd _output_get (delegate Custom|RaceEnd)))

(fn ConstructionScript)