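; BP_NitroHoop is a one-use racing pickup that rewards and boosts a RedisRacerPawn entering its box.
; Overlap shows a W_CacheHit widget and adds time and score through the game mode.
; It also adds velocity along the camera's forward vector and changes SpeedFOV, restoring both after FOVDuration.
; The hoop destroys itself after a short delay, so that restore only runs if FOVDuration elapses first.
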(event OnComponentBeginOverlap(Box)
  (params (OverlappedComponent :type Primitive%20Component%20Object%20Reference) (OtherActor :type Actor%20Object%20Reference) (OtherComp :type Primitive%20Component%20Object%20Reference) (OtherBodyIndex :type Integer) (bFromSweep :type Boolean) (SweepResult :type Hit%20Result%20Structure%20%28by%20ref%29))
  (bind _redisracergamemode (Variables|Default|GetRedisRacerGameMode))
  (bind _asredis_racer_pawn (Utilities|Casting|CastToRedisRacerPawn OtherActor))
  (Utilities|FlowControl|Sequence
    (:then_0
      (bind _returnvalue (UserInterface|CreateWidget "/Game/Blueprints/Widgets/W_CacheHit.W_CacheHit_C"))
      (UserInterface|Viewport|AddtoViewport _returnvalue 0)
      (Default|AddTimeRemaining _redisracergamemode (Variables|Default|GetTimeToAdd))
      (Default|AddScore _redisracergamemode (Variables|Default|GetScoreToAdd)))
    (:then_1
      (bind _output_get (Variables|Default|SetRedisRacerPawn _asredis_racer_pawn))
      (bind _returnvalue_2 (Physics|GetPhysicsLinearVelocity (Variables|/Script/ChaosVehicles.WheeledVehiclePawn|GetMesh _output_get) "None"))
      (Variables|Default|SetLinearVelocity _returnvalue_2)
      (Variables|Default|SetSpeed%20FOV (Variables|/Game/Blueprints/RedisRacerPawn.RedisRacerPawn_C|GetSpeedFOV _output_get))
      (Physics|SetPhysicsLinearVelocity (Variables|/Script/ChaosVehicles.WheeledVehiclePawn|GetMesh _output_get) (* (Transformation|GetActorForwardVector (Game|GetPlayerCameraManager 0)) (Variables|Default|GetSpeedBoost)) true "None")
      (Variables|/Game/Blueprints/RedisRacerPawn.RedisRacerPawn_C|SetSpeedFOV (Variables|Default|GetRedisRacerPawn) (Variables|Default|GetBoost%20FOV))
      (Utilities|FlowControl|Delay (Variables|Default|GetFOVDuration))
      (Physics|SetPhysicsLinearVelocity (Variables|/Script/ChaosVehicles.WheeledVehiclePawn|GetMesh _output_get) (Variables|Default|GetLinearVelocity) false "None")
      (Variables|/Game/Blueprints/RedisRacerPawn.RedisRacerPawn_C|SetSpeedFOV (Variables|Default|GetRedisRacerPawn) (Variables|Default|GetSpeed%20FOV)))
    (:then_2
      (Utilities|FlowControl|Delay 0.2)
      (Actor|DestroyActor))))

(event EventBeginPlay
  (bind _asredis_racer_game_mode (Utilities|Casting|CastToRedisRacerGameMode (Game|GetGameMode)))
  (Variables|Default|SetRedisRacerGameMode _asredis_racer_game_mode))

(fn ConstructionScript)