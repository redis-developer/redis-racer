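; Game mode for a timed driving race that shows the start menu, sets up the race and manages score and time.
; After a countdown delay it shows the vehicle HUD, which Tick feeds with speed, gear and time left.
; A single timer handle serves as the race clock, re-set with extra seconds when time is gained.
; Race end broadcasts win state, initials and score plus remaining milliseconds; timeout counts as a loss.
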(event Custom|RaceEnd
  (params (bWin :type Boolean))
  (bind _tm_timeremaining (Variables|Default|GetTM_TimeRemaining))
  (Default|CallEventRaceEnd bWin (+ (Math|Float|Truncate (* (Utilities|Time|GetTimerRemainingTimebyHandle _tm_timeremaining) 1e+03)) (Variables|Default|GetScore)) (Variables|Default|GetInitials))
  (Utilities|Time|ClearandInvalidateTimerbyHandle _tm_timeremaining))

(event Custom|RaceStart
  (Utilities|FlowControl|Delay (Variables|Default|GetCountdownDuration))
  (UserInterface|Viewport|AddtoViewport (Variables|Default|GetVehicleHUD) 0)
  (bind _returnvalue (Utilities|Time|SetTimerbyEvent (delegate Custom|OutOfTime) 1e+01))
  (Variables|Default|SetTM_TimeRemaining _returnvalue))

(event Custom|OutOfTime
  (CallFunction|RaceEnd false))

(event Custom|RaceSetup
  ;[0.15 0.15 0.15 0.5] Race Setup
  (Utilities|FlowControl|Sequence
    (:then_0
      (bind _asredis_racer_pawn (Utilities|Casting|CastToRedisRacerPawn (Game|Player|GetPlayerPawn 0)))
      (Variables|Default|SetRedisRacerPawn _asredis_racer_pawn))
    (:then_1
      ;;[0.05098 0.05098 0.05098] Create VehicleHUD widget without adding it to the screen
      (bind _returnvalue (UserInterface|CreateWidget "/Game/Blueprints/Widgets/W_VehicleHUD.W_VehicleHUD_C" (Game|GetPlayerController 0) (Variables|/Game/Blueprints/RedisRacerPawn.RedisRacerPawn_C|GetbIsMPH (Variables|Default|GetRedisRacerPawn))))
      (Variables|Default|SetVehicleHUD _returnvalue))
    (:then_2
      ;;[0.15 0.15 0.15 0.5] StartRace
      (CallFunction|RaceStart)
      (Variables|Default|SetbRaceStarted true))))

(event EventTick
  (params (DeltaSeconds :type Float%20%28single-precision%29))
  (bind _redisracerpawn (Variables|Default|GetRedisRacerPawn))
  ;[0.05098 0.05098 0.05098] Update vehicle HUD only after race has started
  (if (Variables|Default|GetbRaceStarted)
    (Default|UpdateSpeed (Variables|Default|GetVehicleHUD) (Variables|/Game/Blueprints/RedisRacerPawn.RedisRacerPawn_C|GetCurrentSpeed _redisracerpawn))
    (Default|UpdateGear (Variables|Default|GetVehicleHUD) (Class|ChaosVehicleMovementComponent|GetCurrentGear (Variables|/Script/ChaosVehicles.WheeledVehiclePawn|GetVehicleMovementComponent _redisracerpawn)))
    (Default|UpdateTimer (Variables|Default|GetVehicleHUD) (Utilities|Time|GetTimerRemainingTimebyHandle (Variables|Default|GetTM_TimeRemaining)))))

(event EventBeginPlay
  ;[0.05098 0.05098 0.05098] BeginPlay: Create StartMenu
  (bind _returnvalue (UserInterface|CreateWidget "/Game/Blueprints/Widgets/W_StartMenu.W_StartMenu_C" (Game|GetPlayerController 0)))
  (UserInterface|Viewport|AddtoViewport _returnvalue 0))

(fn ConstructionScript)

(fn AddTimeRemaining
  (params (TimeToAdd :type Float%20%28double-precision%29))
  (bind _returnvalue (Utilities|Time|SetTimerbyEvent (EventDispatchers|CreateEvent :!event Custom|OutOfTime) (+ TimeToAdd (Utilities|Time|GetTimerRemainingTimebyHandle (Variables|Default|GetTM_TimeRemaining)))))
  (Variables|Default|SetTM_TimeRemaining _returnvalue)
  (Default|TimeGainedAnimation (Variables|Default|GetVehicleHUD)))

(fn AddScore
  (params (ScoreToAdd :type Integer))
  (Variables|Default|SetScore (+ ScoreToAdd (Variables|Default|GetScore))))